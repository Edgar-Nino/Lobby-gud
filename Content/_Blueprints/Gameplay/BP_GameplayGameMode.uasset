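; Multiplayer gameplay game mode that handles player spawning, session cleanup on logout and chat relay.
; SpawnPlayer destroys any controlled pawn, spawns the given class at a random PlayerStart (the last array entry is never picked) and possesses it.
; Controllers registered on OnSwapPlayerControllers receive chat updates through interface messages.
; On logout, it asks the Steam game instance to destroy the exiting controller's session.
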(event `SpawnPlayer`
  (params (PlayerController :type "PlayerController Object Reference") (CharacterClass :type "Character Class Reference"))
  (bind _returnvalue (`Controller.K2_GetPawn` PlayerController))
  (bind _spawnpoints (`self.SpawnPoints`))
  (bind _outactors (`GameplayStatics.GetAllActorsOfClass` "/Script/Engine.PlayerStart"))
  (set `self.SpawnPoints` _outactors)
  (`/Engine/EditorBlueprintResources/StandardMacros.IsValid` _returnvalue
    (:`Is Valid`
      (`KismetSystemLibrary.PrintString` "valid")
      (`self.K2_DestroyActor` _returnvalue))
    (:`Is Not Valid`
      (`KismetSystemLibrary.PrintString` "notvalid")))
  (bind _returnvalue_2 (`|SpawnActorFromClass` CharacterClass (`self.GetTransform` (`|GetArrayItem` _spawnpoints (`KismetMathLibrary.RandomInteger` (- (`KismetArrayLibrary.Array_Length` _spawnpoints) 1)))) "AlwaysSpawn" "OverrideRootScale" null null))
  (`Controller.Possess` PlayerController _returnvalue_2))

(event `self.K2_OnSwapPlayerControllers`
  (params (OldPC :type "PlayerController Object Reference") (NewPC :type "PlayerController Object Reference"))
  (`KismetArrayLibrary.Array_Add` (`self.AllPlayerControllers`) NewPC))

(event `self.K2_OnLogout`
  (params (ExitingController :type "Controller Object Reference"))
  (bind _gameplaypc (message `/Game/_Blueprints/Gameplay/BPI_GameplayPC.GameplayPCref` ExitingController))
  (bind _gameinstance (message `/Game/_Blueprints/BPI_GameInstance.SteamGameInstanceRef` (`GameplayStatics.GetGameInstance`)))
  (message `/Game/_Blueprints/BPI_GameInstance.DestroySessionCaller` _gameinstance _gameplaypc))

(event `UpdateChat`
  (params (Sender :type Text) (Message :type Text))
  (for _array_element (`self.AllPlayerControllers`)
    (bind _gameplaypc (message `/Game/_Blueprints/Gameplay/BPI_GameplayPC.GameplayPCref` _array_element))
    (`/Game/_Blueprints/Gameplay/BP_GameplayPC.UpdateChatWindow` _gameplaypc Sender Message)))

(fn `GameplayGMRef`
  (returns (GameplayGMRef :type "/Game/_Blueprints/Gameplay/BP_GameplayGameMode Object Reference"))
  (return self))

(fn `UserConstructionScript`)