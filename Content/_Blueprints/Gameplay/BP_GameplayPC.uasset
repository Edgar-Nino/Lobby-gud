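; Gameplay player controller that brings in the player's saved character and provides a chat UI.
; On local BeginPlay it loads the PlayerSettingsSave slot and hands the settings to the game mode via an interface to spawn the character, then adds the chat widget after a short delay.
; Chat text and player name go to the game mode, though Sender and Message are swapped, and UpdateChatWindow is empty.
; Enter toggles the mouse cursor.
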(event `self.ReceiveBeginPlay`
  (if (`self.IsLocalController`)
    (`WidgetLayoutLibrary.RemoveAllWidgets`)
    (`self.LoadGame`)))

(event `LoadGame`
  (bind _returnvalue (`GameplayStatics.LoadGameFromSlot` (`self.PlayerSettingsSave`)))
  (bind _asplayer_save (cast `/Game/_Blueprints/PlayerSave` _returnvalue))
  (bind _output_get (set `self.PlayerSettings` (`/Game/_Blueprints/PlayerSave.PlayerInfo` _asplayer_save)))
  (`self.PassCharacterInfoToServer` _output_get))

(event `PassCharacterInfoToServer`
  (params (PlayerSettings :type "/Game/_Blueprints/S_PlayerInfo Structure"))
  (bind _output_get (set `self.PlayerSettings` PlayerSettings))
  (bind _gameplaygmref (message `/Game/_Blueprints/Gameplay/BPI_GameplayGM.GameplayGMRef` (`GameplayStatics.GetGameMode`)))
  (`/Game/_Blueprints/Gameplay/BP_GameplayGameMode.SpawnPlayer` _gameplaygmref self (`.PlayerCharacter_16_6EA448244137B4356C465E9BAE8C4E0F` (break `/Game/_Blueprints/S_PlayerInfo` _output_get)))
  (`KismetSystemLibrary.Delay` 0.2)
  (`self.SetupUI`))

(event `SetupUI`
  (bind _returnvalue (`|CreateWidget` "/Game/_Widgets/ChatGameplay.ChatGameplay_C"))
  (bind _output_get (set `self.GameplayChat` _returnvalue))
  (`UserWidget.AddToViewport` _output_get 0))

(event `GetChatMessage`
  (params (TexToSend :type Text))
  (set `self.SenderText` TexToSend)
  (set `self.SenderName` (`.PlayerName_11_C473324C4A506DEA49AA9EAC1FAC5E34` (break `/Game/_Blueprints/S_PlayerInfo` (`self.PlayerSettings`))))
  (bind _gameplaygmref (message `/Game/_Blueprints/Gameplay/BPI_GameplayGM.GameplayGMRef` (`GameplayStatics.GetGameMode`)))
  (`/Game/_Blueprints/Gameplay/BP_GameplayGameMode.UpdateChat` _gameplaygmref (`self.SenderText`) (`self.SenderName`)))

(event `UpdateChatWindow`
  (params (Sender :type Text) (Message :type Text)))

(event `Key|Enter`
  (params (Key :type "Key Structure"))
  (:`Pressed`
    (`/Engine/EditorBlueprintResources/StandardMacros.FlipFlop`
      (:`A`
        (set `self.bShowMouseCursor` true))
      (:`B`
        (set `self.bShowMouseCursor` false)))))

(fn `GameplayPCref`
  (returns (GameplayPC :type "/Game/_Blueprints/Gameplay/BP_GameplayPC Object Reference"))
  (return self))

(fn `UserConstructionScript`)